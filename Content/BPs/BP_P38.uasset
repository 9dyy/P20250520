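; BP_P38 is a player-controlled plane pawn that flies constantly forward and fires rockets.
; Tick feeds forward movement input scaled by SpeedScale, which the Boost action raises while held.
; Pitch and Roll axes apply clamped, frame-rate independent local rotations, and Fire spawns a BP_Rocket at the Arrow component's transform.
; Both propeller meshes are registered with BPRotateComponent at BeginPlay.
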(event `self.ReceiveBeginPlay`
  (bind _rotcomp (`/Game/BPs/BP_RotateComponent.RotComp` (`self.BP_RotateComponent`)))
  (`KismetArrayLibrary.Array_Add` _rotcomp (`self.PropellerMeshR`))
  (`KismetArrayLibrary.Array_Add` _rotcomp (`self.PropellerMeshL`)))

(event `self.ReceiveTick`
  (params (DeltaSeconds :type "Float (single-precision)"))
  (`self.AddMovementInput` (`self.GetActorForwardVector`) (`self.SpeedScale`)))

(event `InputAxis|Pitch`
  (params (AxisValue :type "Float (single-precision)"))
  (`self.K2_AddActorLocalRotation` (`KismetMathLibrary.MakeRotator` 0.0 (* (`KismetMathLibrary.FClamp` AxisValue -1.0) (`GameplayStatics.GetWorldDeltaSeconds`) (`self.RotSpeed`)))))

(event `InputAxis|Roll`
  (params (AxisValue :type "Float (single-precision)"))
  (`self.K2_AddActorLocalRotation` (`KismetMathLibrary.MakeRotator` (* (`KismetMathLibrary.FClamp` AxisValue -1.0) (`GameplayStatics.GetWorldDeltaSeconds`) (`self.RotSpeed`)))))

(event `InputAction|Boost`
  (params (Key :type "Key Structure"))
  (:`Pressed`
    (set `self.SpeedScale` 1.0))
  (:`Released`
    (set `self.SpeedScale` 0.6)))

(event `InputAction|Fire`
  (params (Key :type "Key Structure"))
  (:`Pressed`
    (`|SpawnActorFromClass` "/Game/BPs/BP_Rocket.BP_Rocket_C" (`SceneComponent.K2_GetComponentToWorld` (`self.Arrow`)) "Undefined" "MultiplyWithRoot" null null)))

(fn `UserConstructionScript`)